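; Clickable aircraft cabin rear door that opens and closes with sound and is locked for takeoff.
; On BeginPlay it binds to the takeoff pulse of CabinManager_BP, which locks the door and closes it if open.
; Clicks on the unlocked mesh play or reverse one timeline that drives its yaw.
; The open status flips only when the timeline finishes.
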(event `self.ReceiveBeginPlay`
  ;[1 1 1] Bind takeoff pulse
  (bind _returnvalue (`GameplayStatics.GetActorOfClass` "/Game/Blueprints/CabinManager_BP.CabinManager_BP_C"))
  (add `CabinManager.TakeOffPulse` _returnvalue (delegate `TakeOffPulse`)))

(event `TakeOffPulse`
  ;[1 1 1] Lock door for takeoff
  (`self.SetLocked` true)
  ;[1 1 1] If door is open, close it
  (if (`self.GetDoorStatus`)
    (`GameplayStatics.PlaySound2D` "/Game/Sounds/DoorClosing.DoorClosing" 1.0 1.0 0.0 null null :!label _label)
    (bind (_direction _opendoorpivot) (`Timeline|Timeline_0` :!label _label_2)
      (:`Update`
        (`SceneComponent.K2_SetWorldRotation` (`self.StaticMesh`) (`KismetMathLibrary.MakeRotator` 0.0 0.0 _opendoorpivot) false false))
      (:`Finished`
        ;[1 1 1] Reverse status
        (`self.SetDoorStatus` (not (`self.GetDoorStatus`)))))))

(event `self.StaticMesh.OnClicked`
  (params (TouchedComponent :type "PrimitiveComponent Object Reference") (ButtonPressed :type "Key Structure"))
  ;[1 1 1] Check not locked
  (bind _returnvalue (`self.GetLocked`))
  (if _returnvalue
    _
    (elif (`self.GetDoorStatus`)
      (goto _label)
      (else
        (`GameplayStatics.PlaySound2D` "/Game/Sounds/DoorOpening.DoorOpening" 1.0 1.25 0.2 null null)
        (goto _label_2 :!via `Reverse`)))))

(fn `UserConstructionScript`)