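; Pax actor Blueprint for an agent that senses other Pax nearby and can show a stat readout.
; On BeginPlay it hands itself to the PaxInfo widget inside its StatInfo component.
; Each Tick it toggles that widget's visibility from GetViewStatInfo and sphere-scans InfluenceRange for other Pax pawns, storing the results for C++.
; A leftover debug print of age group and politeness from PaxState is unconnected.
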(event `self.ReceiveBeginPlay`
  (`self.InitialisePaxWidgetRef`))

(event `self.ReceiveTick`
  (params (DeltaSeconds :type "Float (single-precision)"))
  (`SceneComponent.SetHiddenInGame` (`self.StatInfo`) (not (`self.GetViewStatInfo`)) false)
  ;[1 1 1] Influence Sphere Scan - sends to cpp
  (bind (_outactors _returnvalue) (`KismetSystemLibrary.SphereOverlapActors` (`self.K2_GetActorLocation`) (`self.Influence Range`) (`|MakeArray` (enumliteral `EObjectTypeQuery` "ObjectTypeQuery3")) "/Script/PaxProto.Pax" (`|MakeArray` self :!type "Actor Object Reference"))))

(fn `InitialisePaxWidgetRef`
  (bind _aspax_info (cast `/Game/UI/GameplayUI/PaxInfo` (`WidgetComponent.GetUserWidgetObject` (`self.StatInfo`))))
  (set `/Game/UI/GameplayUI/PaxInfo.PaxRef` self _aspax_info)
  (return))

(fn `UserConstructionScript`)