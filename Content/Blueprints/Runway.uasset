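; Runway actor that animates the runway away during takeoff in response to pulses from CabinManager_BP.
; On BeginPlay it finds the cabin manager and binds to its takeoff and landing events.
; Takeoff waits briefly for the airbridge animation to end, then a timeline drives the runway's world Y/Z location and uniform scale.
; Landing only prints a debug message, with no animation yet.
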(event `self.ReceiveBeginPlay`
  ;[1 1 1] Listen to take off pulse
  (bind _returnvalue (`GameplayStatics.GetActorOfClass` "/Game/Blueprints/CabinManager_BP.CabinManager_BP_C"))
  (add `CabinManager.TakeOffPulse` _returnvalue (delegate `TakeoffRunway`))
  (add `CabinManager.LandingPulse` _returnvalue (delegate `LandingRunway`)))

(event `TakeoffRunway`
  (bind _runway (`self.Runway`))
  ;[1 1 1] Rotate, drop and scale down with takeoff
  ;;[1 1 1] Delay = Last Airbridge Anim End
  (`KismetSystemLibrary.Delay` 1.75)
  (bind (_direction _runwayzheight _runwayydistance _scale) (`Timeline|Takeoff`)
    (:`Update`
      (`SceneComponent.K2_SetWorldLocation` _runway (`KismetMathLibrary.MakeVector` 0.0 _runwayydistance _runwayzheight) false false)
      (`SceneComponent.SetWorldScale3D` _runway (`KismetMathLibrary.MakeVector` _scale _scale _scale)))))

(event `LandingRunway`
  ;[1 1 1] Landing
  (`KismetSystemLibrary.PrintString` "Runway Landing Recieved"))

(fn `UserConstructionScript`)