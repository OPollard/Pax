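; Toilet actor that lets one passenger at a time use it, with an animated, sounding door.
; DoorTrigger overlap admits a Pax_BP targeting TOILET when unoccupied, teleporting it to ToiletTarget and setting its deploy location.
; Tick pins passengers inside CollisionBox and stops their AI movement, then moves them to the door and frees the toilet once their target changes.
; Entry and exit both play the DoorOpening timeline.
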(event `self.ReceiveTick`
  (params (DeltaSeconds :type "Float (single-precision)"))
  (bind _overlappingactors (`PrimitiveComponent.GetOverlappingActors` (`self.CollisionBox`) "/Game/Blueprints/Pax_BP.Pax_BP_C"))
  ;[1 1 1] Get overlapped pax
  (if (!= (`KismetArrayLibrary.Array_Length` _overlappingactors) 0)
    (for _array_element _overlappingactors
      (bind _aspax_bp (cast `/Game/Blueprints/Pax_BP` _array_element))
      ;[1 1 1] Anchor pax to toilet and stop moving
      (`self.K2_SetActorLocation` _aspax_bp (`SceneComponent.K2_GetComponentLocation` (`self.ToiletTarget`)) false false)
      (`Controller.StopMovement` (`AIBlueprintHelperLibrary.GetAIController` _aspax_bp))
      ;[1 1 1] If the desire is to leave, set unoccupied and unhidden
      (if (and (`|EnumInequality` (`Pax.GetTargetPlace` _aspax_bp) "TOILET") (`self.GetOccupied`))
        (`self.K2_SetActorLocation` _aspax_bp (`SceneComponent.K2_GetComponentLocation` (`self.DoorTrigger`)) false false)
        (`self.SetOccupied` false)
        ;[1 1 1] ToiletDoor
        (bind (_direction _doorrotation) (`Timeline|DoorOpening` :!via `PlayFromStart` :!label _label)
          (:`Update`
            (`SceneComponent.K2_SetWorldRotation` (`self.DoorMesh`) (`KismetMathLibrary.MakeRotator` 0.0 0.0 _doorrotation) false false))
          (:`DoorOpening`
            (`GameplayStatics.PlaySound2D` "/Game/Sounds/ToiletDoorOpen.ToiletDoorOpen" 1.0 1.0 0.0 null null))
          (:`DoorClosing`
            (`GameplayStatics.PlaySound2D` "/Game/Sounds/ToiletDoorClose.ToiletDoorClose" 1.0 1.0 0.0 null null)))))))

(event `self.ReceiveBeginPlay`)

(event `self.DoorTrigger.OnComponentBeginOverlap`
  (params (OverlappedComponent :type "PrimitiveComponent Object Reference") (OtherActor :type "Actor Object Reference") (OtherComp :type "PrimitiveComponent Object Reference") (OtherBodyIndex :type Integer) (bFromSweep :type Boolean) (SweepResult :type "HitResult Structure (by ref)"))
  (bind _returnvalue (`SceneComponent.K2_GetComponentLocation` (`self.ToiletTarget`)))
  ;[1 1 1] Actor is pax and wants to go to toilet
  (bind _aspax_bp (cast `/Game/Blueprints/Pax_BP` OtherActor))
  (if (and (`|EnumEquality` (`Pax.GetTargetPlace` _aspax_bp) "TOILET") (`self.ActorHasTag` OtherActor "Pax"))
    (if (not (`self.GetOccupied`))
      ;[1 1 1] Place in toilet and set occupied
      (`self.SetOccupied` true)
      (`self.K2_SetActorLocation` OtherActor _returnvalue false false)
      (`Pax.SetDeployLocation` _aspax_bp _returnvalue)
      (goto _label :!via `PlayFromStart`))))

(fn `UserConstructionScript`)