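; Spawner block that supplies passenger (Pax_BP) actors at its own location for boarding the cabin.
; It spawns the first passenger shortly after BeginPlay, once the airbridge animation finishes.
; When a tagged passenger leaves its Box with the left mouse released, it spawns another if CabinManager_BP reports more than one seat remaining.
; It binds to the cabin manager's takeoff pulse and destroys itself when takeoff starts.
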(event `self.ReceiveBeginPlay`
  ;[1 1 1] Let Airbridge get into position first, airbridge anim is 1 second
  (`KismetSystemLibrary.Delay` 1.1)
  ;[1 1 1] Spawn Pax on box location at begin play
  (`|SpawnActorFromClass` "/Game/Blueprints/Pax_BP.Pax_BP_C" (`self.GetTransform`) "AlwaysSpawn" "OverrideRootScale" null null)
  ;[1 1 1] Remove Spawner Block After TakeOff Initiated
  (bind _returnvalue (`GameplayStatics.GetActorOfClass` "/Game/Blueprints/CabinManager_BP.CabinManager_BP_C"))
  (add `CabinManager.TakeOffPulse` _returnvalue (delegate `TakeOff`)))

(event `TakeOff`
  ;[1 1 1] Remove Spawner Block After TakeOff Initiated
  (`self.K2_DestroyActor`))

(event `self.Box.OnComponentEndOverlap`
  (params (OverlappedComponent :type "PrimitiveComponent Object Reference") (OtherActor :type "Actor Object Reference") (OtherComp :type "PrimitiveComponent Object Reference") (OtherBodyIndex :type Integer))
  ;[1 1 1] Dont Spawn If No Seats Will Be Available
  (bind _returnvalue (`GameplayStatics.GetActorOfClass` "/Game/Blueprints/CabinManager_BP.CabinManager_BP_C"))
  ;[1 1 1] Spawn Pax everytime the mouse is released and the pax is off the box
  (if (and (and (`self.ActorHasTag` OtherActor "Pax") (not (`PlayerController.IsInputKeyDown` (`GameplayStatics.GetPlayerController` 0) "LeftMouseButton"))) (> (`CabinManager.GetRemainingSeats` _returnvalue) 1))
    (`|SpawnActorFromClass` "/Game/Blueprints/Pax_BP.Pax_BP_C" (`self.GetTransform`) "AlwaysSpawn" "OverrideRootScale" null null)))

(fn `UserConstructionScript`)