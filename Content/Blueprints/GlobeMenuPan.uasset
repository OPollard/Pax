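; GlobeMenuPan is the menu globe actor that plays the animated transition from the menu into the FreeFlight level.
; LevelTransition runs the ZoomIn timeline, which moves the globe mesh along Y relative to the camera.
; The timeline's event cues switch tracks on the MenuMusic actor, show the level description, then hide the globe behind a loading screen.
; The level opens after a fixed delay.
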(event `self.ReceiveBeginPlay`
  ;[1 1 1] Set Ref to menu music
  (bind _returnvalue (`GameplayStatics.GetActorOfClass` "/Game/Blueprints/MenuMusic.MenuMusic_C"))
  (set `self.MenuMusicRef` _returnvalue))

(event `LevelTransition`
  (bind _menumusicref (`self.MenuMusicRef`))
  (`SceneComponent.SetHiddenInGame` (`self.StaticMeshComponent`) false false)
  ;[1 1 1] Zoom in
  (bind (_direction _distanceawayfromcamera) (`Timeline|ZoomIn`)
    (:`Update`
      (`SceneComponent.K2_SetWorldLocation` (`self.StaticMeshComponent`) (`KismetMathLibrary.MakeVector` 0.0 _distanceawayfromcamera 15.0) false false))
    (:`RevealCue`
      ;[1 1 1] Level Reveal Media
      (`AudioComponent.Stop` (`/Game/Blueprints/MenuMusic.LevelApproachingMusic` _menumusicref))
      (`AudioComponent.Play` (`/Game/Blueprints/MenuMusic.LevelRevealMusic` _menumusicref) 0.0)
      (bind _returnvalue (`|CreateWidget` "/Game/UI/MenuUI/LevelDescription.LevelDescription_C" (`GameplayStatics.GetPlayerController` 0)))
      (`UserWidget.AddToViewport` _returnvalue 0))
    (:`BuildingExcitementAnim`
      ;[1 1 1] Transition To Level Approach Media
      (`AudioComponent.FadeOut` (`/Game/Blueprints/MenuMusic.StartMenuMusic` _menumusicref) 2.0 0.0 "Linear")
      (`AudioComponent.Play` (`/Game/Blueprints/MenuMusic.LevelApproachingMusic` _menumusicref) 0.0))
    (:`LoadLevelCue`
      ;[1 1 1] Hide Globe
      (`SceneComponent.SetHiddenInGame` (`self.StaticMeshComponent`) true false)
      ;[1 1 1] LoadingScreen/ScoreTargets
      (`WidgetLayoutLibrary.RemoveAllWidgets`)
      (bind _returnvalue_2 (`|CreateWidget` "/Game/UI/MenuUI/LoadingScreen.LoadingScreen_C"))
      (`UserWidget.AddToViewport` _returnvalue_2 0)
      (`KismetSystemLibrary.Delay` 7.0)
      (`GameplayStatics.OpenLevel` "FreeFlight"))))

(fn `UserConstructionScript`)