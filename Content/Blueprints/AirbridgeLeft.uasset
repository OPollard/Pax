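; Left airbridge actor that plays docking and undocking animations with sound and runs a flickering advert screen while docked.
; BeginPlay docks it and binds to CabinManager_BP's takeoff pulse to toggle docking; the landing pulse only prints a message.
; A timeline drives advert flicker, with nested FlipFlops swapping city, tree and broken-screen textures plus a bulb-blow sound.
; FuselageBeacon's 30-second warning starts a timeline that animates door indicator brightness.
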(event `FlickeringAdvert`
  (bind _advert (`self.Advert`))
  (bind _docked (`self.Docked`))
  ;[1 1 1] Flicker light between 1000 and 2500 lumen
  (bind (_direction _intensity) (`Timeline|Flicker`)
    (:`Update`
      (if _docked
        (`LightComponent.SetIntensity` (`self.Advert`) _intensity)))
    (:`ScreenChange`
      (if _docked
        (`/Engine/EditorBlueprintResources/StandardMacros.FlipFlop`
          (:`A`
            (`/Engine/EditorBlueprintResources/StandardMacros.FlipFlop`
              (:`A`
                (`RectLightComponent.SetSourceTexture` _advert "/Game/Images/Icons/CityAdvert.CityAdvert"))
              (:`B`
                (`RectLightComponent.SetSourceTexture` _advert "/Game/Images/Icons/TreeAdvert.TreeAdvert"))))
          (:`B`
            (`RectLightComponent.SetSourceTexture` _advert "/Game/Images/brokenscreen.brokenscreen")))))
    (:`SoundCue`
      (if _docked
        (`GameplayStatics.PlaySound2D` "/Game/Sounds/LightBulbBlow.LightBulbBlow" 1.0 1.0 0.0 null null)))))

(event `self.ReceiveBeginPlay`
  ;[1 1 1] 30 second warning binding for indicator light
  (bind _returnvalue (`GameplayStatics.GetActorOfClass` "/Game/Blueprints/FuselageBeacon.FuselageBeacon_C"))
  (add `/Game/Blueprints/FuselageBeacon.30SecondWarning` _returnvalue (delegate `30SecondWarning`))
  (`self.FlickeringAdvert`)
  ;[1 1 1] Airbridge Animation
  (bind _returnvalue_2 (`GameplayStatics.GetActorOfClass` "/Game/Blueprints/CabinManager_BP.CabinManager_BP_C"))
  (add `CabinManager.TakeOffPulse` _returnvalue_2 (delegate `Bridge_Retraction`))
  (add `CabinManager.LandingPulse` _returnvalue_2 (delegate `Landing Sequence`))
  (`GameplayStatics.PlaySound2D` "/Game/Sounds/AirbridgeMovement.AirbridgeMovement" 1.0 1.0 0.0 null null)
  (`SkeletalMeshComponent.PlayAnimation` (`self.SkeletalMesh`) "/Game/Meshes/Service_Equipment/Airbridge_Anim_Airbridge_Docking.Airbridge_Anim_Airbridge_Docking" false)
  (set `self.Docked` true :!label _label))

(event `Bridge_Retraction`
  (bind _skeletalmesh (`self.SkeletalMesh`))
  ;[1 1 1] Airbridge Animation
  (`GameplayStatics.PlaySound2D` "/Game/Sounds/AirbridgeMovement.AirbridgeMovement" 1.0 1.0 0.0 null null)
  (if (`self.Docked`)
    (`SkeletalMeshComponent.PlayAnimation` _skeletalmesh "/Game/Meshes/Service_Equipment/Airbridge_Anim_Airbridge_Undocking.Airbridge_Anim_Airbridge_Undocking" false)
    (set `self.Docked` false)
    (else
      (`SkeletalMeshComponent.PlayAnimation` _skeletalmesh "/Game/Meshes/Service_Equipment/Airbridge_Anim_Airbridge_Docking.Airbridge_Anim_Airbridge_Docking" false)
      (goto _label))))

(event `30SecondWarning`
  ;[1 1 1] Pulse Brightness when 30 second warning is given
  (bind (_direction _lightintensity) (`Timeline|Timeline_0`)
    (:`Update`
      (`LightComponent.SetIntensity` (`self.DoorIndicatorLight`) _lightintensity))))

(event `Landing Sequence`
  ;[1 1 1] Landing
  (`KismetSystemLibrary.PrintString` "Landing Received Airbridge Left"))

(fn `UserConstructionScript`)