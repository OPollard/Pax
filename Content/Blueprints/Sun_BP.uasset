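; Sun actor that plays a sunrise when the plane cabin takes off.
; On BeginPlay it finds CabinManager_BP and binds to its TakeOffPulse event.
; After a short delay, a timeline animates the light's intensity while RotatingMovement pitches or rolls the sun at a fixed rate for a few seconds, then stops.
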(event `self.ReceiveBeginPlay`
  ;[1 1 1] Listen to takeoff trigger
  (bind _returnvalue (`GameplayStatics.GetActorOfClass` "/Game/Blueprints/CabinManager_BP.CabinManager_BP_C"))
  (add `CabinManager.TakeOffPulse` _returnvalue (delegate `SunRiseTakeOff`)))

(event `SunRiseTakeOff`
  (bind _rotatingmovement (`self.RotatingMovement`))
  ;[1 1 1] Re-enable for sunrise
  (`KismetSystemLibrary.Delay` 1.75)
  (`self.LightAdjustment`)
  ;[1 1 1] RotatewithTakeOff
  (set `RotatingMovementComponent.RotationRate` (struct :`Roll` -22.5) _rotatingmovement)
  (`KismetSystemLibrary.Delay` 4.0)
  (set `RotatingMovementComponent.RotationRate` (struct) _rotatingmovement))

(event `LightAdjustment`
  (bind (_direction _brightness) (`Timeline|Sunbrightness` :`NewTime` 0.0)
    (:`Update`
      (`LightComponent.SetIntensity` (`self.LightComponent`) _brightness))))

(fn `UserConstructionScript`)