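; FuselageBeacon is a beacon actor that signals when the cabin manager's countdown drops below its warning time.
; It finds CabinManager_BP on BeginPlay and enables tick after a short delay, then polls the remaining time until a one-shot flag is set.
; The warning turns the spotlight red, changes its cone and rotation rate, and fires a dispatcher intended to trigger music.
; The beacon destroys itself on the manager's takeoff pulse.
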(event `self.ReceiveBeginPlay`
  ;[1 1 1] Crucial Delay before tick to ensure cabin manager spawns
  (bind _returnvalue (`GameplayStatics.GetActorOfClass` "/Game/Blueprints/CabinManager_BP.CabinManager_BP_C"))
  (bind _output_get (set `self.CabinManagerRef` _returnvalue))
  (add `CabinManager.TakeOffPulse` _output_get (delegate `Takeoff`))
  (`KismetSystemLibrary.Delay` 1.0)
  (`self.SetActorTickEnabled` true))

(event `Takeoff`
  ;[1 1 1] Destroy self
  (`self.K2_DestroyActor`))

(event `self.ReceiveTick`
  (params (DeltaSeconds :type "Float (single-precision)"))
  (bind _cabinmanagerref (`self.CabinManagerRef`))
  ;[1 1 1] Check for 30 second warning then stop tick
  (if (`self.WarningSent`)
    _
    (elif (< (`CabinManager.GetRemainingTime` _cabinmanagerref) (`CabinManager.GetWarningTime` _cabinmanagerref))
      (`self.30 second Warning`))))

(event `30 second Warning`
  (bind _spotlight (`self.SpotLight`))
  ;[1 1 1] Change Lighting and motion
  (set `self.WarningSent` true)
  (`LightComponent.SetLightColor` _spotlight (struct :`R` 1.0 :`A` 1.0) true)
  (`SpotLightComponent.SetInnerConeAngle` _spotlight 60.0)
  (`SpotLightComponent.SetOuterConeAngle` _spotlight 60.0)
  (set `RotatingMovementComponent.RotationRate` (struct :`Yaw` 180.0) (`self.RotatingMovement`))
  ;[1 1 1] Event Delegate to trigger musicbp
  (`self.30SecondWarning`))

(fn `UserConstructionScript`)