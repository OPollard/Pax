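; Right-side airbridge actor that animates docking and undocking with movement sound in response to the cabin's take-off pulse.
; On BeginPlay it docks, binds retraction to CabinManager_BP's pulse and, after a delay, starts the level's AmbientSound.
; Each pulse toggles the Docked flag, stopping or restarting that ambience.
; Both toggle branches play the undocking animation, so docking is only animated at start.
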(event `self.ReceiveBeginPlay`
  (bind _returnvalue (`GameplayStatics.GetActorOfClass` "/Game/Blueprints/CabinManager_BP.CabinManager_BP_C"))
  (add `CabinManager.TakeOffPulse` _returnvalue (delegate `Bridge_Retraction`))
  (`GameplayStatics.PlaySound2D` "/Game/Sounds/AirbridgeMovement.AirbridgeMovement" 1.0 1.0 0.0 null null)
  (`SkeletalMeshComponent.PlayAnimation` (`self.SkeletalMesh`) "/Game/Meshes/Service_Equipment/Airbridge_Anim_Airbridge_Docking.Airbridge_Anim_Airbridge_Docking" false)
  (set `self.Docked` true)
  (bind _returnvalue_2 (`GameplayStatics.GetActorOfClass` "/Script/Engine.AmbientSound"))
  (`KismetSystemLibrary.Delay` 1.5 :!label _label)
  (`AudioComponent.Play` (`AmbientSound.AudioComponent` _returnvalue_2) 0.0))

(event `Bridge_Retraction`
  (bind _skeletalmesh (`self.SkeletalMesh`))
  (`KismetSystemLibrary.Delay` 0.75)
  (`GameplayStatics.PlaySound2D` "/Game/Sounds/AirbridgeMovement.AirbridgeMovement" 1.0 1.0 0.0 null null)
  (if (`self.Docked`)
    (`SkeletalMeshComponent.PlayAnimation` _skeletalmesh "/Game/Meshes/Service_Equipment/Airbridge_Anim_Airbridge_Undocking.Airbridge_Anim_Airbridge_Undocking" false)
    (set `self.Docked` false)
    (`AudioComponent.Stop` (`AmbientSound.AudioComponent` (stale `self.ReceiveBeginPlay` _returnvalue_2)))
    (else
      (`SkeletalMeshComponent.PlayAnimation` _skeletalmesh "/Game/Meshes/Service_Equipment/Airbridge_Anim_Airbridge_Undocking.Airbridge_Anim_Airbridge_Undocking" false)
      (set `self.Docked` true)
      (goto _label))))

(fn `UserConstructionScript`)