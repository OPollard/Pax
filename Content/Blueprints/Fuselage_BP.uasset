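; Aircraft fuselage actor that animates takeoff and landing when CabinManager_BP broadcasts its pulses.
; Takeoff fires delayed audio and engine flames, rotates the mesh by timeline, and catapults unseated Pax_BP passengers on a timeline event.
; A timer then shrinks the flames to cruise thrust, and landing rotates the mesh before destroying them.
; A turbulence timeline is in testing, but its timer loop never runs.
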(event `Turbulence`
  ;[1 1 1] Turbulence - IN TESTING
  (bind (_direction _turbulence) (`Timeline|Timeline` :!via `PlayFromStart`)
    (:`Update`
      (`SceneComponent.K2_SetWorldRotation` (`self.StaticMeshComponent`) (`KismetMathLibrary.MakeRotator` 0.0 _turbulence) false false))))

(event `self.ReceiveBeginPlay`
  ;[1 1 1] Listen for TakeOff Pulse from CabinManager_BP/.cpp
  (bind _returnvalue (`GameplayStatics.GetActorOfClass` "/Game/Blueprints/CabinManager_BP.CabinManager_BP_C"))
  (add `CabinManager.TakeOffPulse` _returnvalue (delegate `TakeOff Sequence`))
  (add `CabinManager.LandingPulse` _returnvalue (delegate `Landing Sequence`))
  (set `self.CabinManagerRef` _returnvalue))

(event `Landing Sequence`
  ;[1 1 1] Landing Sequence
  ;[1 1 1] Landing Fuselage Rotation - 2 seconds
  (bind (_direction _pitch) (`Timeline|LandingRotation`)
    (:`Update`
      (`SceneComponent.K2_SetWorldRotation` (`self.StaticMeshComponent`) (`KismetMathLibrary.MakeRotator` _pitch) false false))
    (:`Finished`
      (`ActorComponent.K2_DestroyComponent` (`self.EngineFlameRight`))
      (`ActorComponent.K2_DestroyComponent` (`self.EngineFlameLeft`)))))

(event `TakeOff Sequence`
  (bind _audio (`self.Audio`))
  ;[1 1 1] DELAY = last airbridge end
  (`KismetSystemLibrary.Delay` 1.75)
  ;[1 1 1] Audio Noise - Takeoff with fade
  (`AudioComponent.Play` _audio 1.0)
  (`AudioComponent.FadeOut` _audio 6.0 0.0 "Linear")
  ;[1 1 1] Flames at max level for 2 seconds then reduce - redirect below
  (`ActorComponent.Activate` (`self.EngineFlameLeft`) false)
  (`ActorComponent.Activate` (`self.EngineFlameRight`) false)
  (`KismetSystemLibrary.K2_SetTimerDelegate` (delegate `ReduceEngineThrust`) 2.0)
  ;[1 1 1] TakeOff Fuselage Rotation - 2 seconds
  (bind (_direction _pitch) (`Timeline|TakeOffRotation`)
    (:`Update`
      (`SceneComponent.K2_SetWorldRotation` (`self.StaticMeshComponent`) (`KismetMathLibrary.MakeRotator` _pitch) false false))
    (:`Catapult`
      ;[1 1 1] Catapult Timing
      (bind _unseatedpax (`CabinManager.GetUnseatedPax` (`self.CabinManagerRef`)))
      (for _array_element _unseatedpax
        (bind _aspax_bp (cast `/Game/Blueprints/Pax_BP` _array_element))
        (`/Game/Blueprints/Pax_BP.Catapult` _aspax_bp)))))

(event `ReduceEngineThrust`
  ;[1 1 1] Reduce Engine To Cruise Over Time
  (bind (_direction _ylocation _yscale) (`Timeline|ThrustDecrease`)
    (:`Update`
      (`SceneComponent.K2_SetWorldTransform` (`self.EngineFlameRight`) (`KismetMathLibrary.MakeTransform` (`KismetMathLibrary.MakeVector` -290.0 _ylocation -50.0) (struct) (`KismetMathLibrary.MakeVector` 1.0 _yscale 1.0)) false false)
      (`SceneComponent.K2_SetWorldTransform` (`self.EngineFlameLeft`) (`KismetMathLibrary.MakeTransform` (`KismetMathLibrary.MakeVector` 290.0 _ylocation -50.0) (struct) (`KismetMathLibrary.MakeVector` 1.0 _yscale 1.0)) false false))))

(fn `UserConstructionScript`)